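; Fire hazard actor that damages overlapping DefaultPawn_BP pawns while it burns.
; SetFire activate and deactivate events switch the particle system and fire sound cue on and off together.
; On actor begin overlap, an active particle system gates heavy damage to each overlapping pawn and an explosion emitter attached to the fire per hit.
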(event OnActivate(SetFire)
  (Components|Activation|Activate (Variables|Emitter|GetParticleSystemComponent) false)
  (Components|Activation|Activate (Variables|Default|GetFire01_Cue) false))

(event OnDeactivate(SetFire)
  (Components|Activation|Deactivate (Variables|Emitter|GetParticleSystemComponent))
  (Components|Activation|Deactivate (Variables|Default|GetFire01_Cue)))

(event Collision|EventActorBeginOverlap
  (params (OtherActor :type Actor%20Object%20Reference))
  (if (Components|Activation|IsActive (Variables|Emitter|GetParticleSystemComponent))
    (for _array_element (Collision|GetOverlappingActors "/Game/DefaultPawn_BP.DefaultPawn_BP_C" :!class /Script/Engine.Actor)
      (Game|Damage|ApplyDamage _array_element 1e+02 0 self)
      (Effects|SpawnEmitterAttached "/Game/StarterContent/Particles/P_Explosion.P_Explosion" (Variables|Emitter|GetParticleSystemComponent) "None" "0, 0,30.000000"))))

(fn ConstructionScript)